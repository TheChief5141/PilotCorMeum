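; BP_Player_Battle_Controller is the player's battle controller, holding the moves available to the player in combat.
; On Possess it looks up three fixed rows in the BT_Player_Moves data table, stores each as its own variable and combines them into MoveList.
; The lookups are chained, so MoveList is built only if all three rows are found.
; The Use_Move event takes a move number but has no logic yet.
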(event Custom|Use_Move
  (params (Move_Number :type BP%20Structure%20TBBS%20Move%20Structure)))

(event EventBeginPlay)

(event EventTick
  (params (DeltaSeconds :type Float%20%28single-precision%29)))

(event EventPossess
  (params (PossessedPawn :type Pawn%20Object%20Reference))
  (bind _returnvalue (Utilities|GetDataTableRow "/Game/Blueprints/Battle/Player/BT_Player_Moves.BT_Player_Moves" "Move_1")
    (:then
      (Variables|Default|SetMove_One _returnvalue)
      (bind _returnvalue_2 (Utilities|GetDataTableRow "/Game/Blueprints/Battle/Player/BT_Player_Moves.BT_Player_Moves" "Move_2")
        (:then
          (Variables|Default|SetMove_Two _returnvalue_2)
          (bind _returnvalue_3 (Utilities|GetDataTableRow "/Game/Blueprints/Battle/Player/BT_Player_Moves.BT_Player_Moves" "Move_3")
            (:then
              (Variables|Default|SetMove_Three _returnvalue_3)
              (Variables|Default|SetMove_List (Utilities|Array|MakeArray (Variables|Default|GetMove_One) (Variables|Default|GetMove_Two) (Variables|Default|GetMove_Three))))))))))

(fn ConstructionScript)