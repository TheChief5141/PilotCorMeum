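; Player character for turn-based battles that sets up battle state and performs moves from a data table.
; BeginPlay sets the overworld controller's state and resets health, but its move-loading function is an empty stub.
; A separate event fills MoveList from BT_Player_Moves rows.
; Use_Move plays the move's timing Level Sequence; healing only prints a message, and the damage formula is unconnected.
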(event Custom|Use_Move
  (params (Move_Number :type BP%20Structure%20TBBS%20Move%20Structure))
  (bind (_attack_name _damage _guard_damage _if_heals _character_animation _ate_animation _class_reference _audio_timing) (Utilities|Struct|BreakBP_Structure_TBBS_Move Move_Number))
  (bind _returnvalue (Sequencer|Player|CreateLevelSequencePlayer _audio_timing))
  (Sequencer|Player|Play _returnvalue :!class /Script/MovieScene.MovieSceneSequencePlayer)
  (Development|PrintString _attack_name)
  ;[1 1 1] Heals if Beer Slide is current move
  (if _if_heals
    (Development|PrintString "Healed!")))

(event Custom|Get_Player_Battle_Move_List
  (bind _outrownames (DataTable|GetDataTableRowNames "/Game/Blueprints/Battle/Player/BT_Player_Moves.BT_Player_Moves"))
  (for _array_element _outrownames
    (bind _returnvalue (Utilities|GetDataTableRow "/Game/Blueprints/Battle/Player/BT_Player_Moves.BT_Player_Moves" _array_element)
      (:then
        (Development|PrintString (.attack_name _returnvalue))
        (Utilities|Array|Add (Variables|Default|GetMove_List) (Utilities|Struct|MakeBP_Structure_TBBS_Move (.attack_name _returnvalue) (.damage _returnvalue) (.guard_damage _returnvalue) (.if_heals _returnvalue) (.character_animation _returnvalue) (.ate_animation _returnvalue) (.class_reference _returnvalue) (.audio_timing _returnvalue)))))))

(event EventBeginPlay
  (CallFunction|GetPlayerBattleMoves)
  (bind _asbp_player_overworld_controller (Utilities|Casting|CastToBP_Player_Overworld_Controller (Game|GetPlayerController 0)))
  (bind _output_get (Variables|Default|SetAs%20BP%20Player%20Overworld%20Controller _asbp_player_overworld_controller))
  (Variables|/Game/Blueprints/Overworld/Player/BP_Player_Overworld_Controller.BP_Player_Overworld_Controller_C|SetPlayer_State _output_get "NewEnumerator3")
  (bind _output_get_2 (Variables|/Game/Blueprints/Overworld/Player/BP_Player_Overworld_Controller.BP_Player_Overworld_Controller_C|SetMax_Health _output_get 1e+02))
  (Variables|/Game/Blueprints/Overworld/Player/BP_Player_Overworld_Controller.BP_Player_Overworld_Controller_C|SetCurrent_Health _output_get _output_get_2))

(event EventTick
  (params (DeltaSeconds :type Float%20%28single-precision%29)))

(fn ConstructionScript)

(fn GetPlayerBattleMoves)