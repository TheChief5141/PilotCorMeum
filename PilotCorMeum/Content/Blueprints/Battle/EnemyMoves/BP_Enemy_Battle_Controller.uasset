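; Enemy AI controller for turn-based battles that loads moves from DT_TBBS_Moves_Enemy on possession and sets health.
; SELECT_MOVE picks a row (RandomInteger max is 0, so always the first) and attacks the player.
; The attack plays the move's timing sequence, then either applies buff/debuff-adjusted damage or raises the buff, depending on the player's timing window.
; Tick can close that window; healing and other fragments are unconnected.
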(event Custom|Attack_Player
  (params (Player%20Controller :type BP%20Player%20Battle%20Controller%20Object%20Reference) (Chosen_Move :type BP%20Structure%20TBBS%20Move%20Structure))
  (bind (_attack_name _damage _guard_damage _if_heals _character_animation _ate_animation _class_reference _audio_timing) (Utilities|Struct|BreakBP_Structure_TBBS_Move Chosen_Move))
  ;[1 1 1] Attack/guard
  (bind _returnvalue (Sequencer|Player|CreateLevelSequencePlayer _audio_timing))
  (Sequencer|Player|Play _returnvalue :!class /Script/MovieScene.MovieSceneSequencePlayer)
  (Variables|Default|SetMove_In_Progress true)
  (if (Variables|/Game/Blueprints/Battle/Player/BP_Player_Battle_Controller.BP_Player_Battle_Controller_C|GetTiming_Window_Active Player%20Controller)
    (bind _output_get (Variables|Default|SetEnemy_Debuff (- (Variables|Default|GetEnemy_Debuff) 1)))
    (Game|Damage|ApplyDamage 0 (Math|Conversions|ToFloat(Integer) (+ (* (+ (stale _output_get_2) _output_get) 4) _damage)) 0 0)
    (else
      (bind _output_get_2 (Variables|Default|SetEnemy_Buff (+ (Variables|Default|GetEnemy_Buff) 1))))))

(event Custom|SELECT_MOVE
  (bind _outrownames (DataTable|GetDataTableRowNames "/Game/Blueprints/Battle/EnemyMoves/DT_TBBS_Moves_Enemy.DT_TBBS_Moves_Enemy"))
  (bind _returnvalue (Utilities|GetDataTableRow "/Game/Blueprints/Battle/EnemyMoves/DT_TBBS_Moves_Enemy.DT_TBBS_Moves_Enemy" (Utilities|Array|Get(acopy) _outrownames (Math|Random|RandomInteger 0)))
    (:then
      (Development|PrintString (.Attack_Name (Utilities|Struct|BreakBP_Structure_TBBS_Move _returnvalue)))
      (bind _output_get (Variables|Default|SetCurrent_Move (Utilities|Struct|MakeBP_Structure_TBBS_Move (.Attack_Name (Utilities|Struct|BreakBP_Structure_TBBS_Move _returnvalue)) (.Damage (Utilities|Struct|BreakBP_Structure_TBBS_Move _returnvalue)) (.Guard_Damage (Utilities|Struct|BreakBP_Structure_TBBS_Move _returnvalue)) (.If_Heals (Utilities|Struct|BreakBP_Structure_TBBS_Move _returnvalue)) (.Character_Animation (Utilities|Struct|BreakBP_Structure_TBBS_Move _returnvalue)) (.ATE_Animation (Utilities|Struct|BreakBP_Structure_TBBS_Move _returnvalue)) (.Class_Reference (Utilities|Struct|BreakBP_Structure_TBBS_Move _returnvalue)) (.Audio_Timing (Utilities|Struct|BreakBP_Structure_TBBS_Move _returnvalue)))))
      (CallFunction|AttackPlayer (Variables|Default|GetAs%20BP%20Player%20Battle%20Controller) _output_get)
      (Variables|Default|SetEnemy_Debuff 0)
      (Variables|Default|SetEnemy_Buff 0))))

(event Custom|Apply_Damage
  (params (Damage_Roll :type Float%20%28double-precision%29)))

(event EventBeginPlay)

(event EventTick
  (params (DeltaSeconds :type Float%20%28single-precision%29))
  (bind _as_bp_player_battle_controller (Variables|Default|GetAs%20BP%20Player%20Battle%20Controller))
  ;[1 1 1] Window Time
  (if (Variables|Default|GetMove_In_Progress)
    (if (Variables|/Game/Blueprints/Battle/Player/BP_Player_Battle_Controller.BP_Player_Battle_Controller_C|GetTiming_Window_Active _as_bp_player_battle_controller)
      (Variables|Default|SetInput_Time (Variables|Default|GetWindow_Time))
      (if (<= (- (Variables|Default|GetInput_Time) DeltaSeconds) 0.0)
        (Variables|/Game/Blueprints/Battle/Player/BP_Player_Battle_Controller.BP_Player_Battle_Controller_C|SetTiming_Window_Active _as_bp_player_battle_controller false)
        (Variables|/Game/Blueprints/Battle/Player/BP_Player_Battle_Controller.BP_Player_Battle_Controller_C|SetCan_Use_Timing_Window _as_bp_player_battle_controller true)))))

(event EventPossess
  (params (PossessedPawn :type Pawn%20Object%20Reference))
  (bind _outrownames (DataTable|GetDataTableRowNames "/Game/Blueprints/Battle/EnemyMoves/DT_TBBS_Moves_Enemy.DT_TBBS_Moves_Enemy"))
  (for _array_element _outrownames
    (bind _returnvalue (Utilities|GetDataTableRow "/Game/Blueprints/Battle/EnemyMoves/DT_TBBS_Moves_Enemy.DT_TBBS_Moves_Enemy" _array_element)
      (:then
        (Utilities|Array|Add (Variables|Default|GetMove_List) _returnvalue)
        (bind _output_get (Variables|Default|SetMax_Health 1e+02))
        (Variables|Default|SetCurrent_Health _output_get)))))

(fn ConstructionScript)