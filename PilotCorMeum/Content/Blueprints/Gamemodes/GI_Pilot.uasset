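; GI_Pilot, apparently the game instance, switches the game between the speakeasy whitebox battle level and the city map.
; Switch_To_Battle opens the level, async-loads the enemy and, if it is a BP_Interactable_Objects, moves it to the enemy spawn's transform, with debug prints.
; Switch_To_City opens the map, waits briefly, then restores the overworld character to LastPlayerLocation.
; Both open levels by name, leaving object-reference variants unwired.
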(event Custom|Switch_To_Battle
  (params (Player_Actor :type Actor%20Object%20Reference) (Enemy_Actor :type Actor%20Soft%20Object%20Reference))
  (Game|OpenLevel(byName) "LVL_SpeakeasyWhitebox")
  (bind _object (Utilities|AsyncLoadAsset Enemy_Actor)
    (:then
      (bind _returnvalue (Actor|GetActorOfClass "/Game/Blueprints/Battle/Spawnpoints/BP_Enemy_Spawn_Location.BP_Enemy_Spawn_Location_C")))
    (:Completed
      (if (Utilities|ClassIsChildOf (Utilities|GetClass _object) "/Game/Blueprints/Overworld/Interactable_Objects/BP_Interactable_Objects.BP_Interactable_Objects_C")
        (Development|PrintString "Hello")
        (bind _asbp_interactable_objects (Utilities|Casting|CastToBP_Interactable_Objects _object))
        (Transformation|SetActorTransform _asbp_interactable_objects (Transformation|GetActorTransform _returnvalue))
        (else
          (Development|PrintString "goodbye"))))))

(event Custom|Switch_To_City
  (params (Player_Actor :type Actor%20Object%20Reference))
  (Game|OpenLevel(byName) "LVL_CityMap")
  (Utilities|FlowControl|Delay 1.0)
  (bind _returnvalue (Actor|GetActorOfClass "/Game/Blueprints/Overworld/Player/BP_Player_Overworld_Character.BP_Player_Overworld_Character_C"))
  (Transformation|SetActorTransform _returnvalue (Variables|Default|GetLast_Player_Location)))