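; BP_Interactable_Objects is an overworld interactable object Blueprint, apparently an early scaffold for player interaction.
; An Interaction event, noted as belonging on the player, sends the BPI_Interaction message to the first array element implementing that interface.
; ObjectInteraction calls the empty RunInteraction event, then prints a debug string if the player pawn overlaps the checked actor.
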(event Custom|Interaction
  ;[1 1 1] Should be placed on player
  (bind _array_element (Utilities|Array|ForEachLoopwithBreak 0 :!label _label)
    (:LoopBody
      (if (Utilities|DoesObjectImplementInterface _array_element "/Game/Blueprints/Overworld/Interactable_Objects/BPI_Interaction.BPI_Interaction_C")
        (Class|BPIInteraction|RunInteraction(Message) _array_element)
        (goto _label Break)))))

(event EventBeginPlay)

(event Collision|EventActorBeginOverlap
  (params (OtherActor :type Actor%20Object%20Reference)))

(event EventTick
  (params (DeltaSeconds :type Float%20%28single-precision%29)))

(event EventRunInteraction
  ;[1 1 1] Interaction
)

(fn ConstructionScript)

(fn ObjectInteraction
  ;[1 1 1] Interaction
  (CallFunction|RunInteraction)
  (if (Collision|IsOverlappingActor (Game|Player|GetPlayerPawn 0) (Variables|Default|GetOther) :!class /Script/Engine.Actor)
    (Development|PrintString "Interaction")))