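; Knife evidence interactable for the overworld that starts a dialogue from the enemy deception table when the player interacts with it.
; On BeginPlay it sets its display name and caches the player's overworld controller.
; Interaction loads every row of DT_Enemy_CDS_Deception into a combat dialogue list, passes it with the name to the controller, then shows the first enemy line and its choices.
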(event Custom|Setup_Combat_Dialogue
  (bind _as_bp_player_overworld_controller (Variables|Default|GetAs%20BP%20Player%20Overworld%20Controller))
  (bind _as_bp_player_overworld_controller_2 (Variables|Default|GetAs%20BP%20Player%20Overworld%20Controller))
  (Variables|/Game/Blueprints/Overworld/Player/BP_Player_Overworld_Controller.BP_Player_Overworld_Controller_C|SetName_Of_Interacted_Object _as_bp_player_overworld_controller (Variables|Default|GetName_Of_Actor))
  (bind _outrownames (DataTable|GetDataTableRowNames "/Game/Blueprints/Dialogue/Combat_Dialogue_System/Enemy/Data_Tables/DT_Enemy_CDS_Deception.DT_Enemy_CDS_Deception"))
  (for _array_element _outrownames
    (bind _returnvalue (Utilities|GetDataTableRow "/Game/Blueprints/Dialogue/Combat_Dialogue_System/Enemy/Data_Tables/DT_Enemy_CDS_Deception.DT_Enemy_CDS_Deception" _array_element)
      (:then
        (Utilities|Array|Add (Variables|Default|GetCombat_Dialogue_List) _returnvalue))))
  (Variables|/Game/Blueprints/Overworld/Player/BP_Player_Overworld_Controller.BP_Player_Overworld_Controller_C|SetEnemy_Combat_Dialogue_Choices _as_bp_player_overworld_controller_2 (Variables|Default|GetCombat_Dialogue_List))
  (Default|DisplayEnemyText _as_bp_player_overworld_controller_2)
  (Default|GetDialogueChoices _as_bp_player_overworld_controller))

(event EventBeginPlay
  (|CallParentFunction)
  (Variables|Default|SetName_Of_Actor "Knifew")
  (bind _asbp_player_overworld_controller (Utilities|Casting|CastToBP_Player_Overworld_Controller (Game|GetPlayerController 0)))
  (Variables|Default|SetAs%20BP%20Player%20Overworld%20Controller _asbp_player_overworld_controller))

(event Collision|EventActorBeginOverlap
  (params (OtherActor :type Actor%20Object%20Reference))
  (|CallParentFunction OtherActor) ; This node is disabled and will not be called.\nDrag off pins to build functionality.
)

(event EventTick
  (params (DeltaSeconds :type Float%20%28single-precision%29))
  (|CallParentFunction DeltaSeconds) ; This node is disabled and will not be called.\nDrag off pins to build functionality.
)

(event EventRunInteraction
  (|CallParentFunction)
  (CallFunction|SetupCombatDialogue))

(fn ConstructionScript
  (|CallParentFunction))