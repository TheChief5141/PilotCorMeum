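; Interactable overworld citizen, the chef Kelso, who starts the Act One Scene One dialogue when interacted with.
; BeginPlay sets the name and caches the overworld player controller.
; Interaction runs the parent logic, then gathers every row of the scene's dialogue DataTable into a list.
; That list is handed to the controller, which displays it from the first entry.
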(event Custom|Setup_Dialogue
  (bind _as_bp_player_overworld_controller (Variables|Default|GetAs%20BP%20Player%20Overworld%20Controller))
  (bind _outrownames (DataTable|GetDataTableRowNames "/Game/Blueprints/Dialogue/Story_Dialogue_System/Data_Tables/Act_One/DT_Dialogue_SDS_Act_One_Scene_One.DT_Dialogue_SDS_Act_One_Scene_One"))
  (for _array_element _outrownames
    (bind _returnvalue (Utilities|GetDataTableRow "/Game/Blueprints/Dialogue/Story_Dialogue_System/Data_Tables/Act_One/DT_Dialogue_SDS_Act_One_Scene_One.DT_Dialogue_SDS_Act_One_Scene_One" _array_element)
      (:then
        (Utilities|Array|Add (Variables|Default|GetDialogue_List) _returnvalue))))
  (Variables|/Game/Blueprints/Overworld/Player/BP_Player_Overworld_Controller.BP_Player_Overworld_Controller_C|SetAct_One_Scene_One_Dialogue_List _as_bp_player_overworld_controller (Variables|Default|GetDialogue_List))
  (Default|DisplayText _as_bp_player_overworld_controller))

(event EventBeginPlay
  (|CallParentFunction)
  (Variables|Default|SetName_Of_Actor "Kelso")
  (bind _asbp_player_overworld_controller (Utilities|Casting|CastToBP_Player_Overworld_Controller (Game|GetPlayerController 0)))
  (Variables|Default|SetAs%20BP%20Player%20Overworld%20Controller _asbp_player_overworld_controller))

(event Collision|EventActorBeginOverlap
  (params (OtherActor :type Actor%20Object%20Reference))
  (|CallParentFunction OtherActor) ; This node is disabled and will not be called.\nDrag off pins to build functionality.
)

(event EventTick
  (params (DeltaSeconds :type Float%20%28single-precision%29))
  (|CallParentFunction DeltaSeconds) ; This node is disabled and will not be called.\nDrag off pins to build functionality.
)

(event EventRunInteraction
  (|CallParentFunction)
  (CallFunction|SetupDialogue))

(fn ConstructionScript
  (|CallParentFunction))