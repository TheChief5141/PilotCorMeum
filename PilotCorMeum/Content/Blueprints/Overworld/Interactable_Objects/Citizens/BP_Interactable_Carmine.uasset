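; Interactable overworld citizen Carmine, whose dialogue comes from the Carmen Act One data table.
; On BeginPlay, after the parent logic, it runs Setup Dialogue, which appends every row of DT_Carmen_SDS_Act_One to DialogueList in row-name order as returned.
; The Blueprint holds no interaction or playback logic of its own, only this data loading.
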(event Custom|Setup_Dialogue
  (bind _outrownames (DataTable|GetDataTableRowNames "/Game/Blueprints/Dialogue/Story_Dialogue_System/Data_Tables/Act_One/Characters/Detectives/DT_Carmen_SDS_Act_One.DT_Carmen_SDS_Act_One"))
  (for _array_element _outrownames
    (bind _returnvalue (Utilities|GetDataTableRow "/Game/Blueprints/Dialogue/Story_Dialogue_System/Data_Tables/Act_One/Characters/Detectives/DT_Carmen_SDS_Act_One.DT_Carmen_SDS_Act_One" _array_element)
      (:then
        (Utilities|Array|Add (Variables|Default|GetDialogue_List) _returnvalue)))))

(event EventBeginPlay
  (|CallParentFunction)
  (CallFunction|SetupDialogue))

(event Collision|EventActorBeginOverlap
  (params (OtherActor :type Actor%20Object%20Reference))
  (|CallParentFunction OtherActor) ; This node is disabled and will not be called.\nDrag off pins to build functionality.
)

(event EventTick
  (params (DeltaSeconds :type Float%20%28single-precision%29))
  (|CallParentFunction DeltaSeconds) ; This node is disabled and will not be called.\nDrag off pins to build functionality.
)

(fn ConstructionScript
  (|CallParentFunction))