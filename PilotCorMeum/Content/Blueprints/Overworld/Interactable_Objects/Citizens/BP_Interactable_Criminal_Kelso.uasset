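; Interactable criminal citizen Kelso in the overworld, who feeds the Act One Scene One dialogue to the player.
; On BeginPlay it runs dialogue setup, which reads every row of the scene's dialogue DataTable into DialogueList.
; For each row found, it copies the growing list to the overworld player controller and calls DisplayText at the first index, independent of interaction.
; RunInteraction only defers to the parent class.
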(event Custom|Setup_Dialogue
  (bind _dialogue_list (Variables|Default|GetDialogue_List))
  (bind _outrownames (DataTable|GetDataTableRowNames "/Game/Blueprints/Dialogue/Story_Dialogue_System/Data_Tables/Act_One/DT_Dialogue_SDS_Act_One_Scene_One.DT_Dialogue_SDS_Act_One_Scene_One"))
  (for _array_element _outrownames
    (bind _returnvalue (Utilities|GetDataTableRow "/Game/Blueprints/Dialogue/Story_Dialogue_System/Data_Tables/Act_One/DT_Dialogue_SDS_Act_One_Scene_One.DT_Dialogue_SDS_Act_One_Scene_One" _array_element)
      (:then
        (Utilities|Array|Add _dialogue_list _returnvalue)
        (bind _asbp_player_overworld_controller (Utilities|Casting|CastToBP_Player_Overworld_Controller (Game|GetPlayerController 0)))
        (Variables|/Game/Blueprints/Overworld/Player/BP_Player_Overworld_Controller.BP_Player_Overworld_Controller_C|SetAct_One_Scene_One_Dialogue_List _asbp_player_overworld_controller _dialogue_list)
        (Default|DisplayText _asbp_player_overworld_controller)))))

(event EventBeginPlay
  (|CallParentFunction)
  (CallFunction|SetupDialogue))

(event Collision|EventActorBeginOverlap
  (params (OtherActor :type Actor%20Object%20Reference))
  (|CallParentFunction OtherActor) ; This node is disabled and will not be called.\nDrag off pins to build functionality.
)

(event EventTick
  (params (DeltaSeconds :type Float%20%28single-precision%29))
  (|CallParentFunction DeltaSeconds) ; This node is disabled and will not be called.\nDrag off pins to build functionality.
)

(event EventRunInteraction
  (|CallParentFunction))

(fn ConstructionScript
  (|CallParentFunction))