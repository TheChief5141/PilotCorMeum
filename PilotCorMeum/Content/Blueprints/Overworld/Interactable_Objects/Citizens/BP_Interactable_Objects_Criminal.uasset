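; Criminal citizen interactable for the overworld that switches the player into another state when interacted with.
; RunInteraction sets its player-state and enemy/player dialogue-system enums, then spawns a new instance of the GameMode's HUD class as Player_HUD_System to add the state's widget to the viewport.
; It then writes the player state and dialogue-system use onto BP_Player_Overworld_Controller.
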(event EventBeginPlay
  (|CallParentFunction) ; This node is disabled and will not be called.\nDrag off pins to build functionality.
)

(event Collision|EventActorBeginOverlap
  (params (OtherActor :type Actor%20Object%20Reference))
  (|CallParentFunction OtherActor) ; This node is disabled and will not be called.\nDrag off pins to build functionality.
)

(event EventTick
  (params (DeltaSeconds :type Float%20%28single-precision%29))
  (|CallParentFunction DeltaSeconds) ; This node is disabled and will not be called.\nDrag off pins to build functionality.
)

(event EventRunInteraction
  (Variables|Default|SetEnemy_Player_Dialogue_System_Use "NewEnumerator2")
  (bind _output_get (Variables|Default|SetBP%20Enum%20Player%20States "NewEnumerator2"))
  (bind _returnvalue (Game|SpawnActorfromClass (Variables|/Script/Engine.GameModeBase|GetHUDClass (Game|GetGameMode)) (Variables|Default|GetSpawn%20Transform) "Undefined" "MultiplyWithRoot" 0 0))
  (bind _asplayer_hud_system (Utilities|Casting|CastToPlayer_HUD_System _returnvalue))
  (Default|AddWBtoViewport _asplayer_hud_system _output_get)
  (bind _asbp_player_overworld_controller (Utilities|Casting|CastToBP_Player_Overworld_Controller (Game|GetPlayerController 0)))
  (Variables|/Game/Blueprints/Overworld/Player/BP_Player_Overworld_Controller.BP_Player_Overworld_Controller_C|SetPlayer_State _asbp_player_overworld_controller "NewEnumerator2")
  (Variables|/Game/Blueprints/Overworld/Player/BP_Player_Overworld_Controller.BP_Player_Overworld_Controller_C|SetEnemy_Player_Dialgoue_System_Use _asbp_player_overworld_controller (Variables|Default|GetEnemy_Player_Dialogue_System_Use)))

(fn ConstructionScript
  (|CallParentFunction))