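; Player controller for the story dialogue system, which creates the dialogue widget and sets Game and UI input when it possesses a pawn.
; It loads three Act One data tables into per-scene lists, then selects the first scene-one line as CurrentDialogueOption.
; IA_Interact requests the line after the stored index, but that index is never incremented here and the other two lists are not read.
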(event Custom|Create_Story_Dialogue_System
  (bind _returnvalue (Game|GetPlayerController 0))
  (bind _returnvalue_2 (UserInterface|CreateWidget "/Game/HUD/WB_SDS_Player.WB_SDS_Player_C" _returnvalue))
  (Input|SetInputModeGameandUI _returnvalue _returnvalue_2 "DoNotLock" true false)
  (bind _output_get (Variables|Default|SetSDS_Widget _returnvalue_2))
  (UserInterface|Viewport|AddtoViewport _output_get 0)
  (bind _outrownames (DataTable|GetDataTableRowNames "/Game/Blueprints/Dialogue/Story_Dialogue_System/Data_Tables/Act_One/DT_Dialogue_SDS_Act_One_Scene_One.DT_Dialogue_SDS_Act_One_Scene_One"))
  (for _array_element _outrownames
    (bind _returnvalue_3 (Utilities|GetDataTableRow "/Game/Blueprints/Dialogue/Story_Dialogue_System/Data_Tables/Act_One/DT_Dialogue_SDS_Act_One_Scene_One.DT_Dialogue_SDS_Act_One_Scene_One" _array_element)
      (:then
        (Utilities|Array|Add (Variables|Default|GetAct_One_Scene_One_Dialogue_List) _returnvalue_3))))
  (bind _outrownames_2 (DataTable|GetDataTableRowNames "/Game/Blueprints/Dialogue/Story_Dialogue_System/Data_Tables/Act_One/Characters/Detectives/DT_Carmen_SDS_Act_One.DT_Carmen_SDS_Act_One"))
  (for _array_element_2 _outrownames_2
    (bind _returnvalue_4 (Utilities|GetDataTableRow "/Game/Blueprints/Dialogue/Story_Dialogue_System/Data_Tables/Act_One/Characters/Detectives/DT_Carmen_SDS_Act_One.DT_Carmen_SDS_Act_One" _array_element_2)
      (:then
        (Utilities|Array|Add (Variables|Default|GetAct_One_Scene_Two_Dialogue_List) _returnvalue_4))))
  (bind _outrownames_3 (DataTable|GetDataTableRowNames "/Game/Blueprints/Dialogue/Story_Dialogue_System/Data_Tables/Act_One/Characters/Enemies/Criminal/DT_Kelso_SDS_Act_One.DT_Kelso_SDS_Act_One"))
  (for _array_element_3 _outrownames_3
    (bind _returnvalue_5 (Utilities|GetDataTableRow "/Game/Blueprints/Dialogue/Story_Dialogue_System/Data_Tables/Act_One/Characters/Enemies/Criminal/DT_Kelso_SDS_Act_One.DT_Kelso_SDS_Act_One" _array_element_3)
      (:then
        (Utilities|Array|Add (Variables|Default|GetAct_One_Scene_Three_Dialogue_List) _returnvalue_5)))))

(event Custom|Display_Text
  (params (Dialogue_Option :type Integer))
  (Variables|Default|SetCurrentDialogueOption (Utilities|Array|Get(acopy) (Variables|Default|GetAct_One_Scene_One_Dialogue_List) Dialogue_Option)))

(event Input|EnhancedActionEvents|EnhancedInputActionIA_Interact
  (params (ActionValue :type Boolean) (ElapsedSeconds :type Float%20%28double-precision%29) (TriggeredSeconds :type Float%20%28double-precision%29) (InputAction :type Input%20Action%20Object%20Reference :default "/Game/Blueprints/Overworld/Input/Actions/IA_Interact.IA_Interact"))
  (:Triggered
    (Development|PrintString "triggered"))
  (:Started
    (Development|PrintString "hehe ha")
    (bind _output_get (Variables|Default|SetCurrent_Dialogue_Option_Index (Variables|Default|GetCurrent_Dialogue_Option_Index)))
    (CallFunction|DisplayText (+ _output_get 1))))

(event EventBeginPlay)

(event EventTick
  (params (DeltaSeconds :type Float%20%28single-precision%29)))

(event EventPossess
  (params (PossessedPawn :type Pawn%20Object%20Reference))
  (CallFunction|CreateStoryDialogueSystem)
  (CallFunction|DisplayText))

(fn ConstructionScript)