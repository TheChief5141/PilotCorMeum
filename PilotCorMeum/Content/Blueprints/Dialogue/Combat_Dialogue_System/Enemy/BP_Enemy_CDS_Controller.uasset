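; Enemy controller for the combat dialogue system that builds the enemy's pool of dialogue choices when it possesses a pawn.
; A switch on dialogue type selects the Intimidation, Deception or Pacification data table and copies each of its rows into DialogueChoices.
; The switch input is fixed to Intimidation, so only that table loads as written.
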(event EventBeginPlay)

(event EventTick
  (params (DeltaSeconds :type Float%20%28single-precision%29)))

(event EventPossess
  (params (PossessedPawn :type Pawn%20Object%20Reference))
  (switch Utilities|FlowControl|Switch|SwitchonBP_Enum_CBS_Dialogue_Types "NewEnumerator0"
    (:NewEnumerator0
      (bind _outrownames (DataTable|GetDataTableRowNames "/Game/Blueprints/Dialogue/Combat_Dialogue_System/Enemy/Data_Tables/DT_Enemy_CDS_Intimidation.DT_Enemy_CDS_Intimidation"))
      (for _array_element _outrownames
        (bind _returnvalue (Utilities|GetDataTableRow "/Game/Blueprints/Dialogue/Combat_Dialogue_System/Enemy/Data_Tables/DT_Enemy_CDS_Intimidation.DT_Enemy_CDS_Intimidation" _array_element)
          (:then
            (Utilities|Array|Add (Variables|Default|GetDialogue_Choices) _returnvalue)))))
    (:NewEnumerator1
      (bind _outrownames_2 (DataTable|GetDataTableRowNames "/Game/Blueprints/Dialogue/Combat_Dialogue_System/Enemy/Data_Tables/DT_Enemy_CDS_Deception.DT_Enemy_CDS_Deception"))
      (for _array_element_2 _outrownames_2
        (bind _returnvalue_2 (Utilities|GetDataTableRow "/Game/Blueprints/Dialogue/Combat_Dialogue_System/Enemy/Data_Tables/DT_Enemy_CDS_Deception.DT_Enemy_CDS_Deception" _array_element_2)
          (:then
            (Utilities|Array|Add (Variables|Default|GetDialogue_Choices) _returnvalue_2)))))
    (:NewEnumerator2
      (bind _outrownames_3 (DataTable|GetDataTableRowNames "/Game/Blueprints/Dialogue/Combat_Dialogue_System/Enemy/Data_Tables/DT_Enemy_CDS_Pacification.DT_Enemy_CDS_Pacification"))
      (for _array_element_3 _outrownames_3
        (bind _returnvalue_3 (Utilities|GetDataTableRow "/Game/Blueprints/Dialogue/Combat_Dialogue_System/Enemy/Data_Tables/DT_Enemy_CDS_Pacification.DT_Enemy_CDS_Pacification" _array_element_3)
          (:then
            (Utilities|Array|Add (Variables|Default|GetDialogue_Choices) _returnvalue_3)))))))

(fn ConstructionScript)