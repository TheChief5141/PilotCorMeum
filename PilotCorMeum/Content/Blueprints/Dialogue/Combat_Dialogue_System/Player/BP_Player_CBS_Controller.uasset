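; Player controller for the combat dialogue phase that hands the pawn over to the turn-based battle controller afterwards.
; On possess it creates the dialogue widget and loads intimidation, deception and pacification lines from three data tables, picking rows by round index.
; Each selection only prints its type and advances the round.
; After three rounds it removes the widget, spawns the game mode's TBBS controller to possess the pawn and destroys itself.
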(event Custom|Get_Dialogue_Choices
  (params (Dialogue_Round :type Integer))
  (CallFunction|GetIntimitdationDialogueChoice Dialogue_Round)
  (CallFunction|GetDeceptionDialogueChoice Dialogue_Round)
  (CallFunction|GetPacificationDialogueChoice Dialogue_Round))

(event Custom|Select_Dialogue_Option
  (params (Dialogue_Type :type BP_Enum_CBS_Dialogue_Types%20Enum :default "NewEnumerator0"))
  (bind _returnvalue (Utilities|String|EnumtoString Dialogue_Type))
  (switch Utilities|FlowControl|Switch|SwitchonBP_Enum_CBS_Dialogue_Types Dialogue_Type
    (:NewEnumerator0
      (Development|PrintString _returnvalue))
    (:NewEnumerator1
      (Development|PrintString _returnvalue))
    (:NewEnumerator2
      (Development|PrintString _returnvalue)))
  (Variables|Default|SetDialogue_Round (+ (Variables|Default|GetDialogue_Round) 1))
  (if (> (Variables|Default|GetDialogue_Round) 2)
    (bind _asbp_gmb_tbbs (Utilities|Casting|CastToBP_GMB_TBBS (Game|GetGameMode)))
    (bind _returnvalue_2 (Game|SpawnActorfromClass (Variables|/Game/Blueprints/Gamemodes/BP_GMB_TBBS.BP_GMB_TBBS_C|GetPlayer_TBBS_Controller _asbp_gmb_tbbs) (Variables|Default|GetSpawn%20Transform) "Undefined" "MultiplyWithRoot" 0 0))
    (Widget|RemovefromParent (Variables|Default|GetCBS_Widget))
    (Pawn|Possess _returnvalue_2 (Game|Player|GetPlayerPawn 0))
    (Actor|DestroyActor)
    (else
      (CallFunction|GetDialogueChoices (Variables|Default|GetDialogue_Round)))))

(event Custom|Get_Deception_Dialogue_Choice
  (params (Dialogue_Round :type Integer))
  (bind _outrownames (DataTable|GetDataTableRowNames "/Game/Blueprints/Dialogue/Data_Tables/DT_CBS_Player_Dialogue_Deception.DT_CBS_Player_Dialogue_Deception"))
  (bind _returnvalue (Utilities|GetDataTableRow "/Game/Blueprints/Dialogue/Data_Tables/DT_CBS_Player_Dialogue_Deception.DT_CBS_Player_Dialogue_Deception" (Utilities|Array|Get(acopy) _outrownames Dialogue_Round))
    (:then
      (Variables|Default|SetDeception_Dialogue_Choice _returnvalue))))

(event Custom|Get_Pacification_Dialogue_Choice
  (params (Dialogue_Round :type Integer))
  (bind _outrownames (DataTable|GetDataTableRowNames "/Game/Blueprints/Dialogue/Data_Tables/DT_CBS_Player_Dialogue_Pacification.DT_CBS_Player_Dialogue_Pacification"))
  (bind _returnvalue (Utilities|GetDataTableRow "/Game/Blueprints/Dialogue/Data_Tables/DT_CBS_Player_Dialogue_Pacification.DT_CBS_Player_Dialogue_Pacification" (Utilities|Array|Get(acopy) _outrownames Dialogue_Round))
    (:then
      (Variables|Default|SetPacification_Dialogue_Choice _returnvalue))))

(event Custom|Get_Intimitdation_Dialogue_Choice
  (params (Dialogue_Round :type Integer))
  (bind _outrownames (DataTable|GetDataTableRowNames "/Game/Blueprints/Dialogue/Data_Tables/DT_CBS_Player_Dialogue_Intimidation.DT_CBS_Player_Dialogue_Intimidation"))
  (bind _returnvalue (Utilities|GetDataTableRow "/Game/Blueprints/Dialogue/Data_Tables/DT_CBS_Player_Dialogue_Intimidation.DT_CBS_Player_Dialogue_Intimidation" (Utilities|Array|Get(acopy) _outrownames Dialogue_Round))
    (:then
      (Variables|Default|SetIntimidation_Dialogue_Choice _returnvalue))))

(event Custom|Setup_CBS
  (bind _returnvalue (Game|GetPlayerController 0))
  (bind _returnvalue_2 (UserInterface|CreateWidget "/Game/HUD/WB_CDS_Player.WB_CDS_Player_C" _returnvalue))
  (bind _output_get (Variables|Default|SetCBS_Widget _returnvalue_2))
  (UserInterface|Viewport|AddtoViewport _output_get 0)
  (Input|SetInputModeGameandUI _returnvalue _returnvalue_2 "DoNotLock" false false))

(event EventBeginPlay)

(event EventTick
  (params (DeltaSeconds :type Float%20%28single-precision%29)))

(event EventPossess
  (params (PossessedPawn :type Pawn%20Object%20Reference))
  (Variables|Default|SetDialogue_Round 0)
  (CallFunction|SetupCBS)
  (CallFunction|GetDialogueChoices))

(fn ConstructionScript)